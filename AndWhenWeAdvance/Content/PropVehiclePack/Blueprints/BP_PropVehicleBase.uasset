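; Base Blueprint for configurable prop vehicles, assembled in the construction script with no active event logic.
; It removes or rotates doors and trunk by open amounts, optionally randomizing doors from a random stream reseeded through a checkbox-style refresh bool.
; It spawns normal or flat wheel meshes at listed transforms.
; An optional dynamic material instance drives paint, dirt and rust on body panels, and a no-glass option swaps glass slots to an empty material.
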(fn `GenerateDoor`
  (bind _frontdoor_l (`self.FrontDoor_L`))
  (bind _frontdoor_r (`self.FrontDoor_R`))
  (bind _backdoor_r (`self.BackDoor_R`))
  (bind _backdoor_l (`self.BackDoor_L`))
  (`|ExecutionSequence`
    (:`then_0`
      (if (`self.RandomizeOpenAmount`)
        (`|ExecutionSequence`
          (:`then_0`
            ;[1 1 1] Randomize Door Angle - Front Right
            (`/Engine/EditorBlueprintResources/StandardMacros.IsValid` (`self.FrontDoor_R`)
              (:`Is Valid`
                (set `self.OpenAmount_FrontRight` (select `bool` (`self.Open_FrontRight`) :`true` (`KismetMathLibrary.RandomFloatInRangeFromStream` 0.0 1.0 (`self.RandomStream`)))))))
          (:`then_1`
            ;[1 1 1] Randomize Door Angle - Front Left
            (`/Engine/EditorBlueprintResources/StandardMacros.IsValid` (`self.FrontDoor_L`)
              (:`Is Valid`
                (set `self.OpenAmount_FrontLeft` (select `bool` (`self.Open_FrontLeft`) :`true` (`KismetMathLibrary.RandomFloatInRangeFromStream` 0.0 1.0 (`self.RandomStream`)))))))
          (:`then_2`
            ;[1 1 1] Randomize Door Angle - Back Left
            (`/Engine/EditorBlueprintResources/StandardMacros.IsValid` (`self.BackDoor_L`)
              (:`Is Valid`
                (set `self.OpenAmount_BackLeft` (select `bool` (`self.Open_BackLeft`) :`true` (`KismetMathLibrary.RandomFloatInRangeFromStream` 0.0 1.0 (`self.RandomStream`)))))))
          (:`then_3`
            ;[1 1 1] Randomize Door Angle - Back Right
            (`/Engine/EditorBlueprintResources/StandardMacros.IsValid` (`self.BackDoor_R`)
              (:`Is Valid`
                (set `self.OpenAmount_BackRight` (select `bool` (`self.Open_BackRight`) :`true` (`KismetMathLibrary.RandomFloatInRangeFromStream` 0.0 1.0 (`self.RandomStream`))))))))))
    (:`then_1`
      (`|ExecutionSequence`
        (:`then_0`
          ;[1 1 1] Set Door Angle - Front Right
          (`/Engine/EditorBlueprintResources/StandardMacros.IsValid` _frontdoor_r
            (:`Is Valid`
              (`SceneComponent.K2_SetRelativeRotation` _frontdoor_r (`KismetMathLibrary.MakeRotator` 0.0 0.0 (`self.GetDoorAngle` true (`self.OpenAmount_FrontRight`))) false false))))
        (:`then_1`
          ;[1 1 1] Randomize Door Angle - Front Left
          (`/Engine/EditorBlueprintResources/StandardMacros.IsValid` _frontdoor_l
            (:`Is Valid`
              (`SceneComponent.K2_SetRelativeRotation` _frontdoor_l (`KismetMathLibrary.MakeRotator` 0.0 0.0 (`self.GetDoorAngle` false (`self.OpenAmount_FrontLeft`))) false false))))
        (:`then_2`
          ;[1 1 1] Randomize Door Angle - Back Right
          (`/Engine/EditorBlueprintResources/StandardMacros.IsValid` _backdoor_r
            (:`Is Valid`
              (`SceneComponent.K2_SetRelativeRotation` _backdoor_r (`KismetMathLibrary.MakeRotator` 0.0 0.0 (`self.GetDoorAngle` true (`self.OpenAmount_BackRight`))) false false))))
        (:`then_3`
          ;[1 1 1] Randomize Door Angle - Back Left
          (`/Engine/EditorBlueprintResources/StandardMacros.IsValid` _backdoor_l
            (:`Is Valid`
              (`SceneComponent.K2_SetRelativeRotation` _backdoor_l (`KismetMathLibrary.MakeRotator` 0.0 0.0 (`self.GetDoorAngle` false (`self.OpenAmount_BackLeft`))) false false))))
        (:`then_4`
          (return))))))

(fn `HandleMaterials`
  (bind _customiseexteriorcolor (`self.CustomiseExteriorColor`))
  (bind _mid (`self.MID`))
  (`|ExecutionSequence`
    (:`then_0`
      (if _customiseexteriorcolor
        (bind _returnvalue (`KismetMaterialLibrary.CreateDynamicMaterialInstance` (`self.DefaultExteriorMIC`)))
        ;[1 1 1] Set dynamic material instance
        (bind _output_get (set `self.MID` _returnvalue))
        (`MaterialInstanceDynamic.SetVectorParameterValue` _output_get "PaintColor" (`self.CarColor`))
        (`MaterialInstanceDynamic.SetScalarParameterValue` _mid "DirtAmount" (`self.DirtAmount`))
        (`MaterialInstanceDynamic.SetScalarParameterValue` _mid "DirtContrast" (`self.DirtContrast`))
        (`MaterialInstanceDynamic.SetVectorParameterValue` _mid "DirtColor" (`self.DirtColor`))
        (`MaterialInstanceDynamic.SetScalarParameterValue` _mid "RustIntensity" (`self.RustIntensity`))
        (`MaterialInstanceDynamic.SetScalarParameterValue` _mid "RustContrast" (`self.RustContrast`))))
    (:`then_1`
      ;[1 1 1] Apply Dynamic Material
      (`PrimitiveComponent.SetMaterial` (`self.BackDoor_L`) 0 (select `bool` _customiseexteriorcolor :`false` (`self.DefaultExteriorMIC`) :`true` (`self.MID`) :!type "MaterialInterface Object Reference"))
      (`PrimitiveComponent.SetMaterial` (`self.FrontDoor_R`) 0 (select `bool` _customiseexteriorcolor :`false` (`self.DefaultExteriorMIC`) :`true` (`self.MID`) :!type "MaterialInterface Object Reference"))
      (`PrimitiveComponent.SetMaterial` (`self.BackDoor_R`) 0 (select `bool` _customiseexteriorcolor :`false` (`self.DefaultExteriorMIC`) :`true` (`self.MID`) :!type "MaterialInterface Object Reference"))
      (`PrimitiveComponent.SetMaterial` (`self.Hood`) 0 (select `bool` _customiseexteriorcolor :`false` (`self.DefaultExteriorMIC`) :`true` (`self.MID`) :!type "MaterialInterface Object Reference"))
      (`PrimitiveComponent.SetMaterial` (`self.Trunk`) 0 (select `bool` _customiseexteriorcolor :`false` (`self.DefaultExteriorMIC`) :`true` (`self.MID`) :!type "MaterialInterface Object Reference"))
      (`PrimitiveComponent.SetMaterial` (`self.FrontDoor_L`) 0 (select `bool` _customiseexteriorcolor :`false` (`self.DefaultExteriorMIC`) :`true` (`self.MID`) :!type "MaterialInterface Object Reference"))
      (`PrimitiveComponent.SetMaterial` (`self.CarFrame`) 0 (select `bool` _customiseexteriorcolor :`false` (`self.DefaultExteriorMIC`) :`true` (`self.MID`) :!type "MaterialInterface Object Reference"))
      (return))))

(fn `SetNoGlass`
  (bind _trunk (`self.Trunk`))
  (bind _backdoor_r (`self.BackDoor_R`))
  (bind _frontdoor_r (`self.FrontDoor_R`))
  (bind _backdoor_l (`self.BackDoor_L`))
  (bind _frontdoor_l (`self.FrontDoor_L`))
  ;[1 1 1] Overwrite glass material for chassis
  (`PrimitiveComponent.SetMaterial` (`self.CarFrame`) 3 "/Game/PropVehiclePack/Materials/M_NoGlassEmpty.M_NoGlassEmpty")
  (`|ExecutionSequence`
    (:`then_0`
      ;[1 1 1] overwrite glass material for all doors
      (`/Engine/EditorBlueprintResources/StandardMacros.IsValid` _backdoor_r
        (:`Is Valid`
          (`PrimitiveComponent.SetMaterial` _backdoor_r 2 "/Game/PropVehiclePack/Materials/M_NoGlassEmpty.M_NoGlassEmpty"))))
    (:`then_1`
      (`/Engine/EditorBlueprintResources/StandardMacros.IsValid` _frontdoor_r
        (:`Is Valid`
          (`PrimitiveComponent.SetMaterial` _frontdoor_r 2 "/Game/PropVehiclePack/Materials/M_NoGlassEmpty.M_NoGlassEmpty"))))
    (:`then_2`
      (`/Engine/EditorBlueprintResources/StandardMacros.IsValid` _backdoor_l
        (:`Is Valid`
          (`PrimitiveComponent.SetMaterial` _backdoor_l 2 "/Game/PropVehiclePack/Materials/M_NoGlassEmpty.M_NoGlassEmpty"))))
    (:`then_3`
      (`/Engine/EditorBlueprintResources/StandardMacros.IsValid` _frontdoor_l
        (:`Is Valid`
          (`PrimitiveComponent.SetMaterial` _frontdoor_l 2 "/Game/PropVehiclePack/Materials/M_NoGlassEmpty.M_NoGlassEmpty"))))
    (:`then_4`
      ;[1 1 1] Empty Trunk glass material if exist
      (`/Engine/EditorBlueprintResources/StandardMacros.IsValid` _trunk
        (:`Is Valid`
          (if (> (`KismetArrayLibrary.Array_Length` (`MeshComponent.GetMaterials` _trunk)) 2)
            (`PrimitiveComponent.SetMaterial` _trunk 2 "/Game/PropVehiclePack/Materials/M_NoGlassEmpty.M_NoGlassEmpty")))))))

(fn `UserConstructionScript`
  (bind _returnvalue (select `bool` (`self.FlatTyres`) :`false` (`self.WheelClass_Normal`) :`true` (`self.WheelClass_Flat`)))
  (if (`self.CLICK-RefreshRandomValues`)
    ;[1 1 1] Refresh Random Values
    (`KismetMathLibrary.SeedRandomStream` (`self.RandomStream`))
    (`KismetSystemLibrary.PrintString` "RandomValueRefresh")
    (set `self.CLICK-RefreshRandomValues` false))
  (`|ExecutionSequence`
    (:`then_0`
      ;[1 1 1] Generate/Rotate Door
      (if (`self.NoDoor`)
        (`ActorComponent.K2_DestroyComponent` (`self.BackDoor_L`))
        (`ActorComponent.K2_DestroyComponent` (`self.FrontDoor_R`))
        (`ActorComponent.K2_DestroyComponent` (`self.BackDoor_R`))
        (`ActorComponent.K2_DestroyComponent` (`self.FrontDoor_L`))
        (else
          (`self.GenerateDoor`))))
    (:`then_1`
      ;[1 1 1] Generate / rotate Trunk
      (`/Engine/EditorBlueprintResources/StandardMacros.IsValid` (`self.Trunk`)
        (:`Is Valid`
          (if (`self.NoTrunk`)
            (`ActorComponent.K2_DestroyComponent` (`self.Trunk`))
            (else
              (`SceneComponent.K2_SetRelativeRotation` (`self.Trunk`) (`KismetMathLibrary.MakeRotator` (`KismetMathLibrary.Lerp` 0.0 90.0 (`self.TrunkOpenAmount`))) false false))))))
    (:`then_2`
      ;[1 1 1] Generate Wheels
      (if (`self.HaveWheels`)
        (for _array_element (`self.WheelsLocation`)
          (if (not (`self.UseDynamicLighting`))
            ;;[1 1 1] Static Lighting
            (bind _returnvalue_2 (`AddComponent|Static Mesh Component_350` :`RelativeTransform` _array_element))
            (`StaticMeshComponent.SetStaticMesh` _returnvalue_2 _returnvalue)
            (else
              ;;[1 1 1] Dynamic Lighting
              (bind _returnvalue_3 (`AddComponent|StaticMeshComponent_0` :`RelativeTransform` _array_element))
              (`StaticMeshComponent.SetStaticMesh` _returnvalue_3 _returnvalue))))))
    (:`then_3`
      (`self.HandleMaterials`))
    (:`then_4`
      (if (`self.NoGlass`)
        (`self.SetNoGlass`)))))