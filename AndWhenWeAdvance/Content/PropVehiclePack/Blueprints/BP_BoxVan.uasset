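; BP_BoxVan is a box van prop vehicle variant that extends its parent's construction script and removes the inherited back doors, trunk and hood components.
; An optional cargo container has two doors whose yaw follows per-door open amounts, mapped to 0–180 degrees and mirrored by side.
; An optional cargo hood copies the car frame's first material.
; All setup runs in the construction script; the event graph is empty.
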(fn `GetCargoDoorAngle`
  (params (Flipped :type Boolean) (Amount :type "Float (double-precision)"))
  (returns (Angle :type "Float (double-precision)"))
  (bind _returnvalue (`KismetMathLibrary.Lerp` 0.0 180.0 Amount))
  (return (`KismetMathLibrary.SelectFloat` (* _returnvalue -1.0) _returnvalue Flipped)))

(fn `UserConstructionScript`
  (`parent.UserConstructionScript`)
  ;[1 1 1] Destroy Backdoor / Trunk / Hood
  (`ActorComponent.K2_DestroyComponent` (`self.BackDoor_L`))
  (`ActorComponent.K2_DestroyComponent` (`self.BackDoor_R`))
  (`ActorComponent.K2_DestroyComponent` (`self.Trunk`))
  (`ActorComponent.K2_DestroyComponent` (`self.Hood`))
  (`|ExecutionSequence`
    (:`then_0`
      ;[1 1 1] Generate Cargo
      (if (`self.HasCargo`)
        (`SceneComponent.K2_SetRelativeRotation` (`self.Container_Door_L`) (`KismetMathLibrary.MakeRotator` 0.0 0.0 (`self.GetCargoDoorAngle` false (`self.CargoDoorOpenAmount_Left`))) false false)
        (`SceneComponent.K2_SetRelativeRotation` (`self.Container_Door_R`) (`KismetMathLibrary.MakeRotator` 0.0 0.0 (`self.GetCargoDoorAngle` true (`self.CargoDoorOpenAmount_Right`))) false false)
        (else
          (`ActorComponent.K2_DestroyComponent` (`self.Container_Frame`))
          (`ActorComponent.K2_DestroyComponent` (`self.Container_Door_L`))
          (`ActorComponent.K2_DestroyComponent` (`self.Container_Door_R`)))))
    (:`then_1`
      ;[1 1 1] Handle Cargo Hood generation and material
      (if (`self.HasCargoHood`)
        (`PrimitiveComponent.SetMaterial` (`self.SM_BoxVan_Hood`) 0 (`PrimitiveComponent.GetMaterial` (`self.CarFrame`) 0))
        (else
          (`ActorComponent.K2_DestroyComponent` (`self.SM_BoxVan_Hood`)))))))